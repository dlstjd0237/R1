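; Player controller that owns the score HUD and shows the game's result screen.
; BeginPlay creates the score widget with a clear score hard-coded to zero, and score and retry-count events update it.
; GameClear and GameOver both show the result widget with a false success flag, and GameClear also spawns a congratulation actor at the pawn.
; ChangePlayer unpossesses, then possesses a Players entry by index.
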(event `self.ReceiveBeginPlay`
  (`|ExecutionSequence`
    (:`then_0`
      (bind _returnvalue (`|CreateWidget` "/Game/UI/WBP_PlayerScore.WBP_PlayerScore_C" self))
      (bind _output_get (set `self.PlayerScoreWidget` _returnvalue))
      (`UserWidget.AddToViewport` _output_get 0))
    (:`then_1`
      (bind _asbp_d1game_mode (cast `/Game/Blueprints/BP_D1GameMode` (`GameplayStatics.GetGameMode`)))
      (`/Game/UI/WBP_PlayerScore.SetClearScore` (`self.PlayerScoreWidget`) 0))))

(event `self.K2_OnScoreChanged`
  (params (NewScore :type Integer))
  (`/Game/UI/WBP_PlayerScore.SetScore` (`self.PlayerScoreWidget`) NewScore))

(event `self.K2_GameClear`
  (`|ExecutionSequence`
    (:`then_0`
      (`self.GameResult` false))
    (:`then_1`
      (`|SpawnActorFromClass` "/Game/UI/BP_Congratulation.BP_Congratulation_C" (`self.GetTransform` (`GameplayStatics.GetPlayerPawn` 0)) "Undefined" "MultiplyWithRoot" null null))))

(event `self.K2_GameOver`
  (`self.GameResult` false))

(event `self.K2_OnGameRetryCount`
  (params (NewRetryCount :type Integer))
  (`/Game/UI/WBP_PlayerScore.SetRetryCount` (`self.PlayerScoreWidget`) NewRetryCount))

(fn `ChangePlayer`
  (params (Index :type Integer))
  (`self.UnPossess`)
  (if (`KismetArrayLibrary.Array_IsValidIndex` (`self.Players`) Index)
    (`self.Possess` (`|GetArrayItem` (`self.Players`) (`local.Index`)))))

(fn `GameResult`
  (params (InSuccess :type Boolean))
  (bind _returnvalue (`|CreateWidget` "/Game/UI/WBP_GameResult.WBP_GameResult_C" self))
  (`UserWidget.AddToViewport` _returnvalue 0)
  (`/Game/UI/WBP_GameResult.SetResult` _returnvalue (`local.InSuccess`)))

(fn `UserConstructionScript`)